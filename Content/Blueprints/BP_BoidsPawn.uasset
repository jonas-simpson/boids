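; BP_BoidsPawn is an observer pawn for a boids scene, providing a smoothly zooming spring-arm camera.
; BeginPlay adds the observer Enhanced Input mapping context, and the zoom action shifts a clamped target distance, printing the raw input value.
; Tick interpolates the current distance toward that target and applies it to the spring arm length.
; The construction script applies the initial distance and seeds the target from it.
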(event Input|EnhancedActionEvents|EnhancedInputActionIA_Zoom
  (params (ActionValue :type Float%20%28double-precision%29) (ElapsedSeconds :type Float%20%28double-precision%29) (TriggeredSeconds :type Float%20%28double-precision%29) (InputAction :type Input%20Action%20Object%20Reference :default "/Game/Input/IA_Zoom.IA_Zoom"))
  (:Triggered
    (Development|PrintString (Utilities|String|ToString(Float) ActionValue))
    (Variables|Default|SetTargetDistance (Math|Float|Clamp(Float) (+ (Variables|Default|GetTargetDistance) (* ActionValue (Variables|Default|GetScrollSpeed))) (Variables|Default|GetDistanceClose) (Variables|Default|GetDistanceFar)))))

(event EventBeginPlay
  (Input|AddMappingContext (PlayerController|LocalPlayerSubsystems|GetEnhancedInputLocalPlayerSubsystem (Game|GetPlayerController 0)) "/Game/Input/IMC_BoidsObserver.IMC_BoidsObserver" 0 "(bIgnoreAllPressedKeysUntilRelease=True,bForceImmediately=False)"))

(event Collision|EventActorBeginOverlap
  (params (OtherActor :type Actor%20Object%20Reference)))

(event EventTick
  (params (DeltaSeconds :type Float%20%28single-precision%29))
  (Variables|Default|SetCamDistance (Math|Interpolation|FInterpTo (Variables|Default|GetCamDistance) (Variables|Default|GetTargetDistance) DeltaSeconds (Variables|Default|GetInterpSpeed)))
  (CallFunction|UpdateCamDistance))

(fn ConstructionScript
  (CallFunction|UpdateCamDistance)
  (Variables|Default|SetTargetDistance (Variables|Default|GetCamDistance)))

(fn UpdateCamDistance
  (Variables|/Script/Engine.SpringArmComponent|SetTargetArmLength (Variables|Default|GetSpringArm) (Variables|Default|GetCamDistance)))