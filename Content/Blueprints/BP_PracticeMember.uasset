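; BP_PracticeMember is a moving actor that holds its own Velocity, apparently one member of a practice group simulation.
; Construction gives it a random direction at fixed speed, and Tick only turns it to face along Velocity.
; SetPosition offsets location by Velocity without delta time and is not called within this Blueprint, as are the Velocity accessors.
; LimitV clamps a vector to MaxSpeed, ignoring its TopSpeed input.
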(event EventBeginPlay)

(event Collision|EventActorBeginOverlap
  (params (OtherActor :type Actor%20Object%20Reference)))

(event EventTick
  (params (DeltaSeconds :type Float%20%28single-precision%29))
  (bind _returnvalue (Transformation|GetActorLocation))
  (Transformation|SetActorRotation (Math|Rotator|FindLookatRotation _returnvalue (+ _returnvalue (Variables|Default|GetVelocity)))))

(fn ConstructionScript
  (Variables|Default|SetVelocity (* (Math|Random|RandomUnitVector) 5.0)))

(fn SetV
  (params (Velocity :type Vector))
  (Variables|Default|SetVelocity Velocity))

(fn GetV
  (return (Variables|Default|GetVelocity)))

(fn SetPosition
  (Transformation|SetActorLocation (+ (Transformation|GetActorLocation) (CallFunction|GetV)) false false))

(fn LimitV
  (params (In%20V :type Vector) (TopSpeed :type Float%20%28double-precision%29))
  (bind _maxspeed (Variables|Default|GetMaxSpeed))
  (bind _output_get (LocalVariables|SetSpeed (Math|Vector|VectorLength In%20V)))
  (if (> _output_get _maxspeed)
    (return (* (Math|Vector|Normalize In%20V) _maxspeed))
    (else
      (return In%20V))))