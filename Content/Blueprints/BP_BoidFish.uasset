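; BP_BoidFish is a fish actor, named as a boid, that varies its size when spawned.
; On BeginPlay it calls the parent, then multiplies the StaticMesh relative scale by one random factor between SizeMin and SizeMax.
; It adds no flocking or movement logic of its own: Tick and overlap events are disabled, and the construction script only calls the parent.
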(event EventBeginPlay
  (bind _staticmesh (Variables|Default|GetStaticMesh))
  (|CallParentFunction)
  (Transformation|SetRelativeScale3D _staticmesh (* (Variables|/Script/Engine.SceneComponent|GetRelativeScale3D _staticmesh) (Math|Random|RandomFloatinRange (Variables|Default|GetSizeMin) (Variables|Default|GetSizeMax)))))

(event Collision|EventActorBeginOverlap
  (params (OtherActor :type Actor%20Object%20Reference))
  (|CallParentFunction OtherActor) ; This node is disabled and will not be called.\nDrag off pins to build functionality.
)

(event EventTick
  (params (DeltaSeconds :type Float%20%28single-precision%29))
  (|CallParentFunction DeltaSeconds) ; This node is disabled and will not be called.\nDrag off pins to build functionality.
)

(fn ConstructionScript
  (|CallParentFunction))