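; BP_PracticeManager is a boids flocking manager, apparently a practice build, that spawns and tracks a population of BP_PracticeMember actors.
; BeginPlay spawns members at random points and rotations inside the Box component's bounds.
; Separation, alignment and cohesion functions each scan all members to compute steering influences.
; Tick calls MoveMembers, but its nested loop is empty; the velocity and position update is disconnected, so the manager moves nothing.
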(event EventBeginPlay
  (CallFunction|InitMembers))

(event Collision|EventActorBeginOverlap
  (params (OtherActor :type Actor%20Object%20Reference)))

(event EventTick
  (params (DeltaSeconds :type Float%20%28single-precision%29))
  (CallFunction|MoveMembers))

(fn ConstructionScript)

(fn InitMembers
  (bind _box (Variables|Default|GetBox))
  (bind (_origin _boxextent) (Collision|GetComponentBounds _box))
  (for _index (range 0 (- (Variables|Default|GetPopulation) 1))
    (bind _returnvalue (Game|SpawnActorfromClass "/Game/Blueprints/BP_PracticeMember.BP_PracticeMember_C" (Math|Transform|MakeTransform (Math|Random|RandomPointinBoundingBox _origin _boxextent) (Math|Random|RandomRotator false)) "Undefined" "MultiplyWithRoot" 0 0))
    (bind _output_get (LocalVariables|SetNewMember _returnvalue))
    (Utilities|Array|Add (Variables|Default|GetMembers) _output_get))
  (return))

(fn MoveMembers
  (bind _members (Variables|Default|GetMembers))
  (for _array_element _members
    (for _array_element_2 _members
      _)))

(fn GetSeparationInfluence
  (params (Member :type BP%20Practice%20Member%20Object%20Reference))
  (for _array_element (Variables|Default|GetMembers)
    ;[1 1 1] Are we looking at ourselves?
    (if (!= Member _array_element)
      ;[1 1 1] Get vector distance to other Boid
      (bind _output_get (LocalVariables|SetDifference (- (Transformation|GetActorLocation _array_element) (Transformation|GetActorLocation Member))))
      ;[1 1 1] If too close,
      (if (< (Math|Float|Absolute(Float) (Math|Vector|VectorLength _output_get)) (Variables|Default|GetDesiredSeparation))
        (LocalVariables|SetInfluence (- (LocalVariables|GetInfluence) (LocalVariables|GetDifference))))))
  (return (LocalVariables|GetInfluence)))

(fn GetAlignmentInfluence
  (params (Member :type BP%20Practice%20Member%20Object%20Reference))
  (for _array_element (Variables|Default|GetMembers)
    (if (!= _array_element Member)
      (LocalVariables|SetPerceivedV (+ (LocalVariables|GetPerceivedV) (Transformation|GetVelocity _array_element)))))
  (bind _output_get (LocalVariables|SetPerceivedV (/ (LocalVariables|GetPerceivedV) (- (Utilities|Array|Length (Variables|Default|GetMembers)) 1))))
  (return (* _output_get (Variables|Default|GetAlignmentScale))))

(fn GetCohesionInfluence
  (params (Member :type BP%20Practice%20Member%20Object%20Reference))
  (for _array_element (Variables|Default|GetMembers)
    (if (!= _array_element Member)
      (LocalVariables|SetPerceivedCenter (+ (LocalVariables|GetPerceivedCenter) (Transformation|GetActorLocation _array_element)))))
  (bind _output_get (LocalVariables|SetPerceivedCenter (/ (LocalVariables|GetPerceivedCenter) (- (Utilities|Array|Length (Variables|Default|GetMembers)) 1))))
  (return (* (- _output_get (Transformation|GetActorLocation Member)) (Variables|Default|GetCohesionScale))))

(fn GetInfluences
  (params (Member :type BP%20Practice%20Member%20Object%20Reference))
  (for _array_element (Variables|Default|GetMembers)
    ;[1 1 1] Are we looking at ourselves?
    (if (!= Member _array_element)
      ;[1 1 1] Get vector distance to other Boid
      (bind _output_get (Variables|Default|SetDifference (- (Transformation|GetActorLocation _array_element) (Transformation|GetActorLocation Member))))
      ;[1 1 1] If too close,
      (if (< (Math|Float|Absolute(Float) (Math|Vector|VectorLength _output_get)) (Variables|Default|GetDesiredSeparation))
        (Variables|Default|SetInfluence (- (Variables|Default|GetInfluence) (Variables|Default|GetDifference))))))
  (return (Variables|Default|GetInfluence)))

(fn GetSeparation
  (params (Member :type BP%20Practice%20Member%20Object%20Reference) (Other :type BP%20Practice%20Member%20Object%20Reference) (Influence%20In :type Vector))
  ;[1 1 1] Get vector distance to other Boid
  (bind _output_get (LocalVariables|SetDifference (- (Transformation|GetActorLocation Other) (Transformation|GetActorLocation Member))))
  ;[1 1 1] If too close,
  (if (< (Math|Float|Absolute(Float) (Math|Vector|VectorLength _output_get)) (Variables|Default|GetDesiredSeparation))
    (return (- Influence%20In (LocalVariables|GetDifference)))))